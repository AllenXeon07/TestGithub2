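; BP_Box is an actor that displays its Number value on two text render components.
; The construction script writes Number as text to both components and colors them green when it is above five, otherwise red.
; All work happens at construction, as the event graph holds only disabled placeholder events.
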(fn `UserConstructionScript`
  (bind _textrender (`self.TextRender`))
  ;[1 1 1] Set Text from Number
  (`TextRenderComponent.K2_SetText` (`self.TextRender`) (`KismetTextLibrary.Conv_IntToText` (`self.Number`)))
  (`TextRenderComponent.K2_SetText` (`self.TextRender1`) (`KismetTextLibrary.Conv_IntToText` (`self.Number`)))
  ;[1 0.2277 0.01702] Change color accord to Number
  (if (> (`self.Number`) 5)
    (`TextRenderComponent.SetTextRenderColor` _textrender (make `Color` 0 255 0 255))
    (`TextRenderComponent.SetTextRenderColor` (`self.TextRender1`) (make `Color` 0 255 0 255))
    (else
      (`TextRenderComponent.SetTextRenderColor` _textrender (make `Color` 0 0 255 255))
      (`TextRenderComponent.SetTextRenderColor` (`self.TextRender1`) (make `Color` 0 0 255 255)))))